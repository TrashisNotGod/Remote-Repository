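; BP_Target is a breakable target that scores when a BP_FireBall hits its Box.
; The hit enables physics on its GeometryCollection, turns off Box collision and calls UpdateScore on BP_ThirdPersonGameMode.
; An IsHit check guards the hit but the flag is only ever set to false, so disabling collision is what blocks repeat hits.
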(event `self.Box.OnComponentHit`
  (params (HitComponent :type "PrimitiveComponent Object Reference") (OtherActor :type "Actor Object Reference") (OtherComp :type "PrimitiveComponent Object Reference") (NormalImpulse :type "Vector Structure") (Hit :type "HitResult Structure (by ref)"))
  (cast `/Game/Blueprints/BP_FireBall` OtherActor)
  (if (not (`self.IsHit`))
    (set `self.IsHit` false)
    (`PrimitiveComponent.SetSimulatePhysics` (`self.GeometryCollection`) true)
    (`PrimitiveComponent.SetCollisionEnabled` (`self.Box`) "NoCollision")
    (bind _asbp_third_person_game_mode (cast `/Game/Blueprints/Player/Blueprints/BP_ThirdPersonGameMode` (`GameplayStatics.GetGameMode`)))
    (`/Game/Blueprints/Player/Blueprints/BP_ThirdPersonGameMode.UpdateScore` _asbp_third_person_game_mode)))

(fn `UserConstructionScript`)