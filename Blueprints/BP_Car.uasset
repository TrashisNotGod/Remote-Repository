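; Car actor that starts moving when the third-person character enters its box, and tracks its own health.
; A one-time overlap calls UpdateTime on the game mode, shows a W_CarHealth widget bound to the car and plays the Move timeline.
; Each timeline update nudges the car along world +Y from its current location, so the curve scales step size rather than absolute position.
; Incoming damage lowers the clamped Health value.
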(event `self.Box.OnComponentBeginOverlap`
  (params (OverlappedComponent :type "PrimitiveComponent Object Reference") (OtherActor :type "Actor Object Reference") (OtherComp :type "PrimitiveComponent Object Reference") (OtherBodyIndex :type Integer) (bFromSweep :type Boolean) (SweepResult :type "HitResult Structure (by ref)"))
  (bind (_returnvalue_x _returnvalue_y _returnvalue_z) (`KismetMathLibrary.BreakVector` (`self.K2_GetActorLocation`)))
  (`/Engine/EditorBlueprintResources/StandardMacros.DoOnce` false
    (:`Completed`
      (cast `/Game/Blueprints/Player/Blueprints/BP_ThirdPersonCharacter` OtherActor)
      (bind _asbp_third_person_game_mode (cast `/Game/Blueprints/Player/Blueprints/BP_ThirdPersonGameMode` (`GameplayStatics.GetGameMode`)))
      (`/Game/Blueprints/Player/Blueprints/BP_ThirdPersonGameMode.UpdateTime` _asbp_third_person_game_mode)
      (bind _returnvalue (`|CreateWidget` "/Game/UI/W_CarHealth.W_CarHealth_C"))
      (`UserWidget.AddToViewport` _returnvalue 0)
      (`/Game/UI/W_CarHealth.SetHealthBar` _returnvalue self)
      (bind (_direction _move) (`Timeline|Move` :!via `PlayFromStart`)
        (:`Update`
          (`self.K2_SetActorLocation` (`KismetMathLibrary.VLerp` (`KismetMathLibrary.MakeVector` _returnvalue_x _returnvalue_y _returnvalue_z) (`KismetMathLibrary.MakeVector` _returnvalue_x (+ _returnvalue_y 4.0) _returnvalue_z) _move)))))))

(event `self.ReceiveAnyDamage`
  (params (Damage :type "Float (single-precision)") (DamageType :type "DamageType Object Reference") (InstigatedBy :type "Controller Object Reference") (DamageCauser :type "Actor Object Reference"))
  (set `self.health` (`KismetMathLibrary.FClamp` (- (`self.health`) Damage) 0.0 200.0)))

(fn `UserConstructionScript`)