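; BP_Enemy_Axe is an axe-wielding enemy that sets up its health and health-bar widget on BeginPlay.
; A fast looping timer caches the axe's begin and end trace-point world positions as attack endpoints.
; BattleCry raises its damage and health up to fixed caps.
; On death, it awards experience and coins to the controlled PlayerCharacter, then calls Buff and Die.
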(event `self.ReceiveBeginPlay`
  ;[1 1 1] Initialize & Update AttackPos
  (bind _output_get (set `self.MaxHealth` 100.0))
  (set `self.Health` _output_get)
  (`self.Initialize`)
  (`KismetSystemLibrary.K2_SetTimerDelegate` (delegate `CustomEvent`) 0.01 true))

(event `CustomEvent`
  ;[1 1 1] Initialize & Update AttackPos
  (set `self.BeginPos` (`SceneComponent.K2_GetComponentLocation` (`self.AxeBeginTracePos`)))
  (set `self.EndPos` (`SceneComponent.K2_GetComponentLocation` (`self.AxeEndTracePos`))))

(event `BattleCry`
  ;[1 1 1] BattleCry
  (set `self.BaseDamage` (`KismetMathLibrary.FClamp` (+ (`self.BaseDamage`) 10.0) 0.0 50.0))
  (set `self.Health` (`KismetMathLibrary.FClamp` (+ (`self.Health`) 50.0) 0.0 200.0)))

(event `self.OnDeath`
  (bind _asplayer_character (cast `PlayerCharacter` (`Controller.K2_GetPawn` (`GameplayStatics.GetPlayerController` 0))))
  (set `PlayerCharacter.Experience` (+ (`PlayerCharacter.Experience` _asplayer_character) 40) _asplayer_character)
  (set `PlayerCharacter.Coins` (+ (`PlayerCharacter.Coins` _asplayer_character) 2) _asplayer_character)
  (`self.Buff`)
  (`self.Die`))

(fn `UserConstructionScript`
  (`parent.UserConstructionScript`))