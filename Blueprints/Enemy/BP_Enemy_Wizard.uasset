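; BP_Enemy_Wizard is an enemy caster that sets up its health and health bar on spawn and fights the player with two attacks.
; Its normal attack fires a fireball aimed at the player, and a trigger box toggles a ChangeSkill flag while the player is inside.
; Its area attack sphere-traces to damage the player, with shockwave, sound and camera shake.
; On death it grants experience and coins, then calls Buff and Die.
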(event `self.ReceiveBeginPlay`
  (bind _output_get (set `self.MaxHealth` 80.0))
  (set `self.Health` _output_get)
  (`self.Initialize`))

(event `Fire!`
  (bind _returnvalue (`SceneComponent.K2_GetComponentLocation` (`self.MagicPos`)))
  ;[1 1 1] NormalAttack
  (`|SpawnActorFromClass` "/Game/Blueprints/BP_FireBall_EnemyWizard.BP_FireBall_EnemyWizard_C" (`KismetMathLibrary.MakeTransform` _returnvalue (`KismetMathLibrary.FindLookAtRotation` _returnvalue (`self.K2_GetActorLocation` (`GameplayStatics.GetPlayerCharacter` 0)))) "Undefined" "MultiplyWithRoot" null null))

(event `self.BoxForChanging.OnComponentBeginOverlap`
  (params (OverlappedComponent :type "PrimitiveComponent Object Reference") (OtherActor :type "Actor Object Reference") (OtherComp :type "PrimitiveComponent Object Reference") (OtherBodyIndex :type Integer) (bFromSweep :type Boolean) (SweepResult :type "HitResult Structure (by ref)"))
  ;[1 1 1] ChangeSkill
  (cast `/Game/Blueprints/Player/Blueprints/BP_ThirdPersonCharacter` OtherActor)
  (set `self.ChangeSkill?` true))

(event `self.BoxForChanging.OnComponentEndOverlap`
  (params (OverlappedComponent :type "PrimitiveComponent Object Reference") (OtherActor :type "Actor Object Reference") (OtherComp :type "PrimitiveComponent Object Reference") (OtherBodyIndex :type Integer))
  ;[1 1 1] ChangeSkill
  (cast `/Game/Blueprints/Player/Blueprints/BP_ThirdPersonCharacter` OtherActor)
  (set `self.ChangeSkill?` false))

(event `AreaAttack`
  (bind _returnvalue (`SceneComponent.K2_GetComponentLocation` (`self.MagicPos`)))
  ;[1 1 1] AreaAttack
  (bind _outactors (`GameplayStatics.GetAllActorsOfClass` null))
  (bind (_outhit _returnvalue_2) (`KismetSystemLibrary.SphereTraceSingle` _returnvalue _returnvalue 550.0 "TraceTypeQuery3" false _outactors))
  (if (and _returnvalue_2 (not (`self.IsDead`)))
    (bind _asbp_third_person_character (cast `/Game/Blueprints/Player/Blueprints/BP_ThirdPersonCharacter` (`.HitActor` (`GameplayStatics.BreakHitResult` _outhit)))
      (:`then`
        (`GameplayStatics.ApplyDamage` _asbp_third_person_character 30.0 null null "/Script/Engine.DamageType"))
      (:`CastFailed`
        _)))
  (`GameplayStatics.SpawnEmitterAtLocation` "/Game/Assets/Characters/Enemy_BOSS/FX/Particles/Abilities/Ultimate/FX/P_Execute_Roar_Shockwave.P_Execute_Roar_Shockwave" (`self.K2_GetActorLocation`))
  (`GameplayStatics.PlaySoundAtLocation` "/Game/Assets/Audio/Stomp.Stomp" (`self.K2_GetActorLocation`) (struct) 1.0 1.0 0.0 null null null null)
  (`GameplayStatics.PlayWorldCameraShake` "/Game/Blueprints/BP_CameraShake_Attack.BP_CameraShake_Attack_C" (0.0 0.0 0.0) 0.0 2000.0))

(event `self.OnDeath`
  (bind _asplayer_character (cast `PlayerCharacter` (`Controller.K2_GetPawn` (`GameplayStatics.GetPlayerController` 0))))
  (set `PlayerCharacter.Experience` (+ (`PlayerCharacter.Experience` _asplayer_character) 40) _asplayer_character)
  (set `PlayerCharacter.Coins` (+ (`PlayerCharacter.Coins` _asplayer_character) 2) _asplayer_character)
  (`self.Buff`)
  (`self.Die`))

(fn `UserConstructionScript`
  (`parent.UserConstructionScript`))