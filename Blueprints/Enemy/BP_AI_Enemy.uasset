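; AI controller for an enemy that starts chasing the third-person player character on sight.
; It runs its behavior tree on BeginPlay and uses PawnSensing to detect pawns.
; When the seen pawn is BP_ThirdPersonCharacter, it stores it and writes the chase flag and player reference to the blackboard.
; The chase flag is never cleared here.
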(event `self.ReceiveBeginPlay`
  (`self.RunBehaviorTree` (`self.BT`)))

(event `self.PawnSensing.OnSeePawn`
  (params (Pawn :type "Pawn Object Reference"))
  (bind _returnvalue (`AIBlueprintHelperLibrary.GetBlackboard` null))
  (bind _asbp_third_person_character (cast `/Game/Blueprints/Player/Blueprints/BP_ThirdPersonCharacter` Pawn))
  (set `self.Player` _asbp_third_person_character)
  (`BlackboardComponent.SetValueAsBool` _returnvalue "StartChasing?" true)
  (`BlackboardComponent.SetValueAsObject` _returnvalue "Player" (`self.Player`)))

(fn `UserConstructionScript`)