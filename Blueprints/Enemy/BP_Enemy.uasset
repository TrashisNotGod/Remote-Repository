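; Melee enemy that takes damage, turns toward the player inside a trigger box and attacks with a sword.
; Montage-driven or direct hits update health, briefly show a health bar widget and set the chase Blackboard key; zero health ragdolls and destroys it.
; Looping timers drive facing and sword sphere traces between two tracked points, ignoring other enemies and throttling damage with a delayed DoOnce reset.
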(event `self.ReceiveBeginPlay`
  ;[1 1 1] Initialize & Update AttackPos
  (`self.Initialize`)
  (`KismetSystemLibrary.K2_SetTimerDelegate` (delegate `UpdatePos`) 0.01 true))

(event `UpdatePos`
  ;[1 1 1] Initialize & Update AttackPos
  (set `self.BeginPos` (`SceneComponent.K2_GetComponentLocation` (`self.BeginTracePos`)))
  (set `self.EndPos` (`SceneComponent.K2_GetComponentLocation` (`self.EndTracePos`))))

(event `self.ReceiveAnyDamage`
  (params (Damage :type "Float (single-precision)") (DamageType :type "DamageType Object Reference") (InstigatedBy :type "Controller Object Reference") (DamageCauser :type "Actor Object Reference"))
  ;[1 1 1] Health System
  (bind _output_get (set `self.Health` (`KismetMathLibrary.FClamp` (- (`self.Health`) Damage) 0.0 (`self.MaxHealth`))))
  (if (== _output_get 0.0)
    (`self.Die`)
    (else
      (if (not (`self.IsAttacking?`))
        (`|PlayMontage` (`self.Mesh`) "/Game/Assets/Animations/Combat/HitReact_Montage.HitReact_Montage"
          (:`then`
            _)))
      (`SceneComponent.SetVisibility` (`self.Widget`) true false)
      (`BlackboardComponent.SetValueAsBool` (`AIBlueprintHelperLibrary.GetBlackboard` null) "StartChasing?" true)
      (`KismetSystemLibrary.Delay` 1.0)
      (`SceneComponent.SetVisibility` (`self.Widget`) false false))))

(event `Die`
  ;[1 1 1] Health System
  (`PrimitiveComponent.SetSimulatePhysics` (`self.Mesh`) true)
  (`ActorComponent.Deactivate` (`self.CharacterMovement`))
  (set `self.IsDead?` true)
  (`PrimitiveComponent.SetCollisionResponseToChannel` (`self.CapsuleComponent`) "ECC_Pawn" "ECR_Ignore")
  (`KismetSystemLibrary.Delay` 1.0)
  (`self.K2_DestroyActor`))

(event `self.BoxForFacing.OnComponentBeginOverlap`
  (params (OverlappedComponent :type "PrimitiveComponent Object Reference") (OtherActor :type "Actor Object Reference") (OtherComp :type "PrimitiveComponent Object Reference") (OtherBodyIndex :type Integer) (bFromSweep :type Boolean) (SweepResult :type "HitResult Structure (by ref)"))
  ;[1 1 1] FacePlayer
  (if (not (`self.IsDead?`))
    (bind _asbp_third_person_character (cast `/Game/Blueprints/Player/Blueprints/BP_ThirdPersonCharacter` OtherActor))
    (set `self.Player` _asbp_third_person_character)
    (bind _returnvalue (`KismetSystemLibrary.K2_SetTimerDelegate` (delegate `FacePlayer`) 0.01 true))
    (set `self.FacePlayerTimehandle` _returnvalue)))

(event `FacePlayer`
  (bind (_returnvalue_roll _returnvalue_pitch _returnvalue_yaw) (`KismetMathLibrary.BreakRotator` (`KismetMathLibrary.FindLookAtRotation` (`self.K2_GetActorLocation`) (`self.K2_GetActorLocation` (`self.Player`)))))
  ;[1 1 1] FacePlayer
  (`self.K2_SetActorRotation` (`KismetMathLibrary.MakeRotator` 0.0 0.0 _returnvalue_yaw)))

(event `self.BoxForFacing.OnComponentEndOverlap`
  (params (OverlappedComponent :type "PrimitiveComponent Object Reference") (OtherActor :type "Actor Object Reference") (OtherComp :type "PrimitiveComponent Object Reference") (OtherBodyIndex :type Integer))
  ;[1 1 1] FacePlayer
  (cast `/Game/Blueprints/Player/Blueprints/BP_ThirdPersonCharacter` OtherActor)
  (`KismetSystemLibrary.K2_ClearAndInvalidateTimerHandle` (`self.FacePlayerTimehandle`)))

(event `EndTrace`
  ;[1 1 1] SwordAttack
  (`KismetSystemLibrary.K2_ClearAndInvalidateTimerHandle` (stale `BeginTrace` _returnvalue)))

(event `/Game/Blueprints/BPI_Damage.BeginSwordTrace`
  ;[1 1 1] SwordAttack
  (`self.BeginTrace`))

(event `BeginTrace`
  ;[1 1 1] SwordAttack
  (bind _returnvalue (`KismetSystemLibrary.K2_SetTimerDelegate` (delegate `DamageTrace`) 0.01 true)))

(event `/Game/Blueprints/BPI_Damage.EndSwordTrace`
  ;[1 1 1] SwordAttack
  (`self.EndTrace`))

(event `DamageTrace`
  ;[1 1 1] SwordAttack
  (bind _outactors (`GameplayStatics.GetAllActorsOfClass` "BP_Enemy_C"))
  (bind (_outhit _returnvalue) (`KismetSystemLibrary.SphereTraceSingle` (`self.BeginPos`) (`self.EndPos`) (`self.Radius`) "TraceTypeQuery3" false _outactors "ForOneFrame"))
  (if (and _returnvalue (not (`self.IsDead?`)))
    (`/Engine/EditorBlueprintResources/StandardMacros.DoOnce` false :!label _label
      (:`Completed`
        (bind _asbp_third_person_character (cast `/Game/Blueprints/Player/Blueprints/BP_ThirdPersonCharacter` (`.HitActor` (`GameplayStatics.BreakHitResult` _outhit))))
        (`GameplayStatics.ApplyDamage` _asbp_third_person_character (`self.Base Damage`) null null "/Script/Engine.DamageType")
        (`KismetSystemLibrary.Delay` 0.5)
        (goto _label :!via `Reset`)))))

(fn `BeginDamageTrace`)

(fn `GetMovementDirection`
  (params (InputAction :type "InputAction Object Reference"))
  (returns (DirectionKey :type "Key Structure"))
  (bind _returnvalue (message `EnhancedInputSubsystemInterface.QueryKeysMappedToAction` (pcsubsystem `EnhancedInputLocalPlayerSubsystem` (`GameplayStatics.GetPlayerController` 0)) InputAction))
  (for _array_element _returnvalue
    (if (`PlayerController.IsInputKeyDown` (`GameplayStatics.GetPlayerController` 0) _array_element)
      (return _array_element))))

(fn `UserConstructionScript`)