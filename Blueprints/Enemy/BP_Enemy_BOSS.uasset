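; Boss enemy that has a high health pool, an area attack and its own on-screen health bar shown on trigger overlap.
; A fast looping timer refreshes attack trace positions, while BigAttack sphere-traces around a socket point, ignores other enemies, damages the player and plays shake and particle effects.
; Death grants experience and coins, calls Buff, flags the boss defeated in the game mode, then hides and relocates it.
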(event `self.ReceiveBeginPlay`
  ;[1 1 1] Initialize & Update AttackPos
  (bind _output_get (set `self.MaxHealth` 300.0))
  (set `self.Health` _output_get)
  (`self.Initialize`)
  (`KismetSystemLibrary.K2_SetTimerDelegate` (delegate `UpdatePos`) 0.005 true))

(event `UpdatePos`
  ;[1 1 1] Initialize & Update AttackPos
  (set `self.BeginPos` (`SceneComponent.K2_GetComponentLocation` (`self.BossBeginTracePos`)))
  (set `self.EndPos` (`SceneComponent.K2_GetComponentLocation` (`self.BossEndTracePos`))))

(event `BigAttack`
  (bind _returnvalue (`SceneComponent.K2_GetComponentLocation` (`self.EndTracePos`)))
  ;[1 1 1] BigAttack
  (bind _outactors (`GameplayStatics.GetAllActorsOfClass` "/Game/Blueprints/Enemy/BP_Enemy.BP_Enemy_C"))
  (bind (_outhit _returnvalue_2) (`KismetSystemLibrary.SphereTraceSingle` _returnvalue _returnvalue 400.0 "TraceTypeQuery3" false _outactors))
  (if (and _returnvalue_2 (not (`self.IsDead`)))
    (bind _asbp_third_person_character (cast `/Game/Blueprints/Player/Blueprints/BP_ThirdPersonCharacter` (`.HitActor` (`GameplayStatics.BreakHitResult` _outhit))))
    (`GameplayStatics.ApplyDamage` _asbp_third_person_character 50.0 null null "/Script/Engine.DamageType"))
  (`GameplayStatics.PlayWorldCameraShake` "/Game/Blueprints/BP_CameraShake_Attack.BP_CameraShake_Attack_C" (0.0 0.0 0.0) 0.0 2000.0)
  (`GameplayStatics.SpawnEmitterAtLocation` "/Game/Assets/Characters/Enemy_BOSS/FX/Particles/Abilities/HardKnocks/FX/P_Hardknocks_AOE.P_Hardknocks_AOE" (`self.K2_GetActorLocation`)))

(event `self.UITrigger.OnComponentBeginOverlap`
  (params (OverlappedComponent :type "PrimitiveComponent Object Reference") (OtherActor :type "Actor Object Reference") (OtherComp :type "PrimitiveComponent Object Reference") (OtherBodyIndex :type Integer) (bFromSweep :type Boolean) (SweepResult :type "HitResult Structure (by ref)"))
  ;[1 1 1] BossHealthUITrigger
  (cast `/Game/Blueprints/Player/Blueprints/BP_ThirdPersonCharacter` OtherActor)
  (bind _returnvalue (`|CreateWidget` "/Game/UI/W_BossHealth.W_BossHealth_C"))
  (`UserWidget.AddToViewport` _returnvalue 1)
  (`/Game/UI/W_BossHealth.SetHealthBar` _returnvalue self))

(event `self.Die`
  ;[1 1 1] Die
  (`/Engine/EditorBlueprintResources/StandardMacros.DoOnce` false
    (:`Completed`
      (`|PlayMontage` (`self.Mesh`) "/Game/Assets/Characters/Enemy_BOSS/Characters/Heroes/Grux/Animations/Death_A_Montage.Death_A_Montage"
        (:`then`
          (set `self.IsDead` true)
          (`ActorComponent.Deactivate` (`self.CharacterMovement`))
          (bind _asbp_third_person_game_mode (cast `/Game/Blueprints/Player/Blueprints/BP_ThirdPersonGameMode` (`GameplayStatics.GetGameMode`)))
          (set `/Game/Blueprints/Player/Blueprints/BP_ThirdPersonGameMode.BossDefeated?` true _asbp_third_person_game_mode))
        (:`OnNotifyBegin`
          (`SceneComponent.SetVisibility` (`self.Mesh`) false true)
          (`self.K2_SetActorLocation` (10000.0 0.0 0.0)))))))

(event `self.OnDeath`
  (bind _asplayer_character (cast `PlayerCharacter` (`Controller.K2_GetPawn` (`GameplayStatics.GetPlayerController` 0))))
  (set `PlayerCharacter.Experience` (+ (`PlayerCharacter.Experience` _asplayer_character) 80) _asplayer_character)
  (set `PlayerCharacter.Coins` (+ (`PlayerCharacter.Coins` _asplayer_character) 4) _asplayer_character)
  (`self.Buff`)
  (`self.Die`))

(fn `UserConstructionScript`
  (`parent.UserConstructionScript`))